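; CoinTrigger is a pickup trigger that awards a coin to the 2DSideScrollerCharacter that overlaps it.
; On begin overlap, if CanCollect is set, it destroys its attach parent actor, increments the character's Coins and clears the flag so it pays out only once.
; The end overlap event only casts to the character and takes no further action.
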(event `self.ReceiveActorEndOverlap`
  (params (OtherActor :type "Actor Object Reference"))
  (cast `/Game/2DSideScrollerBP/Blueprints/2DSideScrollerCharacter` OtherActor))

(event `self.ReceiveActorBeginOverlap`
  (params (OtherActor :type "Actor Object Reference"))
  (bind _as2dside_scroller_character (cast `/Game/2DSideScrollerBP/Blueprints/2DSideScrollerCharacter` OtherActor))
  (if (`self.CanCollect`)
    (`self.K2_DestroyActor` (`self.GetAttachParentActor`))
    (bind _output_get (set `self.PlayerVar` _as2dside_scroller_character))
    (`/Engine/EditorBlueprintResources/StandardMacros.IncrementInt` (`/Game/2DSideScrollerBP/Blueprints/2DSideScrollerCharacter.Coins` _output_get)
      (:`  `
        (set `self.CanCollect` false)))))

(fn `UserConstructionScript`)