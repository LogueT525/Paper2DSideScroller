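; EnemyHurtbox is a collision volume that damages the 2D side-scroller player character on contact.
; On begin overlap it casts the other actor to 2DSideScrollerCharacter and subtracts PercentToTake from that character's PlayerHealth.
; When health reaches zero or below, it destroys the player and opens the MainMenu level.
; A health print-out remains in the graph but is disconnected and never runs.
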(event `self.CollisionComponent.OnComponentBeginOverlap`
  (params (OverlappedComponent :type "PrimitiveComponent Object Reference") (OtherActor :type "Actor Object Reference") (OtherComp :type "PrimitiveComponent Object Reference") (OtherBodyIndex :type Integer) (bFromSweep :type Boolean) (SweepResult :type "HitResult Structure (by ref)"))
  (bind _as2dside_scroller_character (cast `/Game/2DSideScrollerBP/Blueprints/2DSideScrollerCharacter` OtherActor))
  (bind _output_get (set `self.PlayerVar` _as2dside_scroller_character))
  (bind _output_get_2 (set `/Game/2DSideScrollerBP/Blueprints/2DSideScrollerCharacter.PlayerHealth` (- (`/Game/2DSideScrollerBP/Blueprints/2DSideScrollerCharacter.PlayerHealth` _output_get) (`self.PercentToTake`)) _output_get))
  (if (<= _output_get_2 0.0)
    (`self.K2_DestroyActor` (`self.PlayerVar`))
    (`GameplayStatics.OpenLevel` "MainMenu")))

(fn `UserConstructionScript`)